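; BP_DebugInteractor is a debug interactable that grants or charges score when a PlayerCharacter interacts with it.
; On interact it calls the parent handler, casts the interactor to PlayerCharacter, then branches on InteractionType.
; Gainable adds Cost to the player's score and destroys the owner; any other type destroys the owner only if the player can spend Cost.
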(event EventBeginPlay)

(event EventTick
  (params (DeltaSeconds :type Float%20%28single-precision%29)))

(event EventOnInteract
  (params (Interactor :type Actor%20Object%20Reference))
  (bind _returnvalue (Components|GetOwner))
  (bind _cost (Variables|Default|GetCost))
  (|CallParentFunction Interactor)
  (bind _asplayer_character (Utilities|Casting|CastToPlayerCharacter Interactor))
  (if (Utilities|Enum|Equal(Enum) (Variables|Default|GetInteractionType) "Gainable")
    (Class|PlayerCharacter|GainScore _asplayer_character _cost)
    (Actor|DestroyActor _returnvalue)
    (else
      (bind _returnvalue_2 (Class|PlayerCharacter|TryUseScore _asplayer_character _cost))
      (if _returnvalue_2
        (Actor|DestroyActor _returnvalue)))))