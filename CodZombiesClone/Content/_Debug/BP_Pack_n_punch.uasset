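; BP_Pack_n_punch is a debug Pack-n-Punch actor whose audio turns on and off with power from a linked electrical switch.
; On BeginPlay it plays or stops its audio according to IsActive, then binds to the switch instance's power-triggered event if that reference is valid.
; Each trigger calls TriggerActive, which toggles both the audio and the IsActive flag.
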(event Custom|OnPowerTriggered
  ;[0.15 0.15 0.15 0.5] Listen to Electrical Switch
  (CallFunction|TriggerActive))

(event EventBeginPlay
  (bind _electricalswitchinstance (Variables|Default|GetElectricalSwitchInstance))
  ;[0.15 0.15 0.15 0.5] Setup start state
  (if (Variables|Default|GetbIsActive)
    (Audio|Components|Audio|Play (Variables|Default|GetAudio) 0.0)
    (else
      (Audio|Components|Audio|Stop (Variables|Default|GetAudio))))
  ;[0.15 0.15 0.15 0.5] Listen to Electrical Switch
  (Utilities|IsValid _electricalswitchinstance
    (:Is%20Valid
      (EventDispatchers|BindEventtoOnPowerTriggered _electricalswitchinstance (delegate Custom|OnPowerTriggered)))))

(fn ConstructionScript)

(fn TriggerActive
  (if (Variables|Default|GetbIsActive)
    (Audio|Components|Audio|Stop (Variables|Default|GetAudio))
    (else
      (Audio|Components|Audio|Play (Variables|Default|GetAudio) 0.0)))
  (Variables|Default|SetbIsActive (not (Variables|Default|GetbIsActive))))