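; Base actor for perk machines that can be switched between powered and unpowered states.
; On BeginPlay it sets its audio and spotlight intensity and color from IsActive, then binds to the power-triggered event of an optional electrical switch instance.
; Each power trigger calls ToggleActive, which flips IsActive and swaps the sound and light to match.
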(event Custom|OnPowerTriggered
  ;[0.15 0.15 0.15 0.5] Listen to Electrical Switch
  (CallFunction|ToggleActive))

(event EventBeginPlay
  (bind _electricalswitchinstance (Variables|Default|GetElectricalSwitchInstance))
  ;[0.15 0.15 0.15 0.5] Setup begin state
  (if (Variables|Default|GetbIsActive)
    (Audio|Components|Audio|Play (Variables|Default|GetAudio) 0.0)
    (Rendering|Components|Light|SetIntensity (Variables|Default|GetSpotLight) (Variables|Default|GetOnIntensity))
    (Rendering|Components|Light|SetLightColor (Variables|Default|GetSpotLight) (Variables|Default|GetActiveColor) true)
    (else
      (Audio|Components|Audio|Stop (Variables|Default|GetAudio))
      (Rendering|Components|Light|SetIntensity (Variables|Default|GetSpotLight) (Variables|Default|GetOffIntensity))
      (Rendering|Components|Light|SetLightColor (Variables|Default|GetSpotLight) (Variables|Default|GetDisabledColor) true)))
  ;[0.15 0.15 0.15 0.5] Listen to Electrical Switch
  (Utilities|IsValid _electricalswitchinstance
    (:Is%20Valid
      (EventDispatchers|BindEventtoOnPowerTriggered _electricalswitchinstance (delegate Custom|OnPowerTriggered)))))

(fn ConstructionScript)

(fn ToggleActive
  (if (Variables|Default|GetbIsActive)
    (Audio|Components|Audio|Stop (Variables|Default|GetAudio))
    (Rendering|Components|Light|SetIntensity (Variables|Default|GetSpotLight) (Variables|Default|GetOffIntensity))
    (Rendering|Components|Light|SetLightColor (Variables|Default|GetSpotLight) (Variables|Default|GetDisabledColor) true)
    (else
      (Audio|Components|Audio|Play (Variables|Default|GetAudio) 0.0)
      (Rendering|Components|Light|SetIntensity (Variables|Default|GetSpotLight) (Variables|Default|GetOnIntensity))
      (Rendering|Components|Light|SetLightColor (Variables|Default|GetSpotLight) (Variables|Default|GetActiveColor) true)))
  (Variables|Default|SetbIsActive (not (Variables|Default|GetbIsActive))))