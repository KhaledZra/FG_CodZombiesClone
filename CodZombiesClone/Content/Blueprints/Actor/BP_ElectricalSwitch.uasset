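; BP_ElectricalSwitch is an electrical lever switch actor that controls whether its linked lights flicker, which they do while the switch is inactive.
; BeginPlay sets the lever rotation and light states from IsActive.
; OnSwitchTriggered plays a timeline that always rotates the lever from off to on.
; On finish, TriggerSwitch toggles the state, snaps the lever and updates the lights, then two Niagara effects activate and OnPowerTriggered is broadcast.
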(event Custom|OnSwitchTriggered
  (bind _leveralpha (Timeline|TL_Lever PlayFromStart)
    (:Update
      (Transformation|SetRelativeRotation (Variables|Default|GetSM_ElectricLever) (Math|Rotator|Lerp(Rotator) (Variables|Default|GetRL_LeverOffRotation) (Variables|Default|GetRL_LeverOnRotation) _leveralpha) false false))
    (:Finished
      (CallFunction|TriggerSwitch)
      (Components|Activation|Activate (Variables|Default|GetNS_EffectLeft) false)
      (Components|Activation|Activate (Variables|Default|GetNS_EffectRight) false)
      (Default|CallOnPowerTriggered))))

(event EventBeginPlay
  (if (Variables|Default|GetbIsActive)
    (Transformation|SetRelativeRotation (Variables|Default|GetSM_ElectricLever) (Variables|Default|GetRL_LeverOnRotation) false false)
    (else
      (Transformation|SetRelativeRotation (Variables|Default|GetSM_ElectricLever) (Variables|Default|GetRL_LeverOffRotation) false false)))
  (for _array_element (Variables|Default|GetLights)
    (Default|SetLightFlicker _array_element (not (Variables|Default|GetbIsActive)))))

(fn ConstructionScript)

(fn TriggerSwitch
  (if (Variables|Default|GetbIsActive)
    (Transformation|SetRelativeRotation (Variables|Default|GetSM_ElectricLever) (Variables|Default|GetRL_LeverOffRotation) false false)
    (else
      (Transformation|SetRelativeRotation (Variables|Default|GetSM_ElectricLever) (Variables|Default|GetRL_LeverOnRotation) false false)))
  (Variables|Default|SetbIsActive (not (Variables|Default|GetbIsActive)))
  (for _array_element (Variables|Default|GetLights)
    (Default|SetLightFlicker _array_element (not (Variables|Default|GetbIsActive)))))