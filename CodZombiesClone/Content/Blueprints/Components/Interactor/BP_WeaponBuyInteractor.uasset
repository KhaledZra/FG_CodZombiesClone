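; Interactor component that sells a weapon to the interacting player character in exchange for score.
; On interact, it checks that a weapon class is set and that the player's current score covers the cost.
; It then tries to equip the weapon and deducts the score only if equipping succeeds.
; Failure cases for an unset class, insufficient score or failed equip only print debug strings.
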(event EventOnInteract
  (params (Interactor :type Actor%20Object%20Reference))
  (if (Utilities|IsValidClass (Variables|Default|GetWeaponClass))
    (bind _asplayer_character (Utilities|Casting|CastToPlayerCharacter Interactor))
    (if (>= (Class|PlayerCharacter|GetCurrentScore _asplayer_character) (Variables|Default|GetCost))
      (bind _returnvalue (Class|PlayerCharacter|TryEquipWeapon _asplayer_character (Variables|Default|GetWeaponClass) (Variables|Default|GetWeaponData)))
      (if _returnvalue
        (Class|PlayerCharacter|TryUseScore _asplayer_character (Variables|Default|GetCost))
        (else
          (Development|PrintString "Maybe already owned?")))
      (else
        (Development|PrintString "Ur broke")))
    (else
      (Development|PrintString "Weapon Class not set"))))