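; BP_WeaponPackNPunch is an interactor that lets the player pay score to upgrade their current weapon, in the style of a Pack-a-Punch machine.
; On begin interact it casts the interactor to PlayerCharacter and checks the current score against Cost.
; It calls TryUpgradeWeapon on the held weapon and deducts Cost only if that succeeds.
; Insufficient score, max level or a failed cast only prints a debug string.
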(event EventOnBeginInteract
  (params (Interactor :type Actor%20Object%20Reference))
  (bind _asplayer_character (Utilities|Casting|CastToPlayerCharacter Interactor)
    (:then
      (if (>= (Class|PlayerCharacter|GetCurrentScore _asplayer_character) (Variables|Default|GetCost))
        (bind _returnvalue (Class|BaseWeapon|TryUpgradeWeapon (Variables|/Script/CodZombiesClone.PlayerCharacter|GetCurrentWeapon _asplayer_character)))
        (if _returnvalue
          (Class|PlayerCharacter|TryUseScore _asplayer_character (Variables|Default|GetCost))
          (else
            (Development|PrintString "Max Level")))
        (else
          (Development|PrintString "Ur broke"))))
    (:CastFailed
      (Development|PrintString "ERROR"))))