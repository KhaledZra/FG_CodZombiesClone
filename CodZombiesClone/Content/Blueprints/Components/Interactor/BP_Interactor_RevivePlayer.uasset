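; Interactor component on a player character that lets another player revive it with a timed interaction.
; Beginning interaction puts the reviver into its revive state, updates accumulate delta time, and stopping resets the timer and ends that state.
; Once the required time is reached, it deactivates itself, awards score to the reviver and revives its owner.
; The prompt appends percentage progress while active and is blank when inactive.
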(event EventOnBeginInteract
  (params (Interactor :type Actor%20Object%20Reference))
  (Variables|Default|SetCurrentInteractTime 0.0)
  (if (Variables|Default|GetbInteractorActive)
    (bind _asplayer_character (Utilities|Casting|CastToPlayerCharacter Interactor)
      (:then
        (bind _output_get (Variables|Default|SetAs%20Player%20Character _asplayer_character))
        (Variables|Default|SetbInteractionCompleted false)
        (Class|PlayerCharacter|StartReviveOtherPlayer _output_get))
      (:CastFailed
        (Class|InteractorComponent|OnStopInteract)))))

(event EventOnStopInteract
  (params (Interactor :type Actor%20Object%20Reference))
  (bind _as_player_character (Variables|Default|GetAs%20Player%20Character))
  (Variables|Default|SetCurrentInteractTime 0.0)
  (Utilities|IsValid _as_player_character
    (:Is%20Valid
      (Class|PlayerCharacter|FinishedReviveOtherPlayer _as_player_character))))

(event EventOnUpdateInteract
  (params (Interactor :type Actor%20Object%20Reference))
  (if (and (Variables|Default|GetbInteractorActive) (== (Variables|Default|GetbInteractionCompleted) false))
    (bind _output_get (Variables|Default|SetCurrentInteractTime (+ (Utilities|Time|GetWorldDeltaSeconds) (Variables|Default|GetCurrentInteractTime))))
    (if (>= _output_get (Variables|Default|GetInteractTimeRequired))
      (Variables|Default|SetbInteractionCompleted true)
      (Variables|Default|SetbInteractorActive false)
      (Class|PlayerCharacter|GainScore (Variables|Default|GetAs%20Player%20Character) 500)
      (bind _asplayer_character (Utilities|Casting|CastToPlayerCharacter (Components|GetOwner)))
      (Class|PlayerCharacter|RevivePlayer _asplayer_character)
      (Development|PrintString "TARGET REVIVED"))))

(fn GetInteractString
  (params (InputKeyText :type Text%20%28by%20ref%29))
  (bind _returnvalue (|CallParentFunction InputKeyText))
  (if (Variables|Default|GetbInteractorActive)
    (if (> (Variables|Default|GetCurrentInteractTime) 0.1)
      (return (Utilities|String|Append _returnvalue " - " (Utilities|String|ToString(Integer) (Class|KismetMathLibrary|ToInt64(Float) (* (/ (Variables|Default|GetCurrentInteractTime) (Variables|Default|GetInteractTimeRequired)) 1e+02))) "%"))
      (else
        (return _returnvalue)))
    (else
      (return ""))))