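; BP_GM_Fps is an FPS game mode that ends the match when no players are left alive and supports adding local players.
; Tick uses a Delay to poll the alive player actors about once a second while the game is active.
; An empty result triggers the game-over message and sound, then reopens Lvl_NightOfTheUndead after a pause.
; The P key creates another local player, capped at four.
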(event EventBeginPlay
  (Variables|Default|SetbGameActive true))

(event EventTick
  (params (DeltaSeconds :type Float%20%28single-precision%29))
  (if (Variables|Default|GetbGameActive)
    (Utilities|FlowControl|Delay 1.0)
    (bind _returnvalue (Class|FpsGameMode|GetAlivePlayerActors))
    (if (Utilities|Array|IsEmpty _returnvalue)
      (Development|PrintString "Game over :(")
      (Variables|Default|SetbGameActive false)
      (Audio|PlaySound2D "/Game/Audio/ZombieSounds/GameOver.GameOver" 1.0 1.0 0.0 0 0)
      (Utilities|FlowControl|Delay 1e+01)
      (Game|OpenLevel(byObjectReference) "/Game/Levels/Lvl_NightOfTheUndead.Lvl_NightOfTheUndead"))))

(event Input|KeyboardEvents|P
  (params (Key :type Key%20Structure :default "None"))
  (:Pressed
    (if (<= (Class|GameplayStatics|GetNumLocalPlayerControllers) 3)
      (Class|GameplayStatics|CreatePlayer -1)
      (else
        (Development|PrintString "Reached Player Limit!")))))

(fn ConstructionScript)